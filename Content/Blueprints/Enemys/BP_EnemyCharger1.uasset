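; BP_EnemyCharger1 is an enemy that chases the first-person player on sight and deals fixed damage to any actor it overlaps.
; Pawn sensing triggers AI MoveTo toward the player, while incoming damage lowers Health and destroys the enemy at zero.
; Each tick yaws the widget health bar toward the player pawn and sets it to a constant fill that does not read Health.
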(event OnSeePawn(PawnSensing)
  (params (Pawn :type Pawn%20Object%20Reference))
  (bind _asfirst_person_character (Utilities|Casting|CastToFirstPersonCharacter Pawn))
  (AI|AIMoveTo self "0, 0, 0" _asfirst_person_character 5.0 false))

(event Collision|EventActorBeginOverlap
  (params (OtherActor :type Actor%20Object%20Reference))
  (Class|BPDamage|TakeDamage(Message) OtherActor 1e+01))

(event EventTakeDamage
  (params (Damage :type Float%20%28single-precision%29))
  (bind _output_get (Variables|Default|SetHealth (- (Variables|Default|GetHealth) Damage)))
  (if (<= _output_get 0.0)
    (Actor|DestroyActor)))

(event EventTick
  (params (DeltaSeconds :type Float%20%28single-precision%29))
  (bind _ashealth_enemy (Utilities|Casting|CastToHealthEnemy (UserInterface|GetUserWidgetObject (Variables|Default|GetWidget))))
  (Progress|SetPercent (Variables|/Game/Blueprints/Dañoyvida/HealthEnemy.HealthEnemy_C|GetVidaEnemy _ashealth_enemy) (/ 25.0 1e+02))
  (Transformation|SetWorldRotation (Variables|Default|GetWidget) (Math|Rotator|MakeRotator 0.0 0.0 (.Yaw (Math|Rotator|BreakRotator (Math|Rotator|FindLookatRotation (Transformation|GetWorldLocation (Variables|Default|GetWidget)) (Transformation|GetActorLocation (Game|Player|GetPlayerPawn 0)))))) false false))

(fn ConstructionScript)