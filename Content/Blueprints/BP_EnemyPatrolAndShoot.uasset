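; Enemy actor that shoots at a sensed first-person player and is destroyed when damage depletes its health.
; PawnSensing turns it toward the player and launches a projectile along the cube's forward vector, with a flag and delay as cooldown.
; BeginPlay stores three patrol points and picks one at random.
; The timeline meant to lerp toward that point and re-pick has nothing triggering it in the graph.
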(event OnSeePawn(PawnSensing)
  (params (Pawn :type Pawn%20Object%20Reference))
  ;[1 1 1] Mirar y Disparar
  (bind _asfirst_person_character (Utilities|Casting|CastToFirstPersonCharacter Pawn))
  (Utilities|FlowControl|Sequence
    (:then_0
      (Transformation|SetActorRotation (Math|Rotator|FindLookatRotation (Transformation|GetActorLocation) (Transformation|GetActorLocation _asfirst_person_character))))
    (:then_1
      (if (Variables|Default|GetProyectilSpawn)
        (bind _returnvalue (Game|SpawnActorfromClass "/Game/FirstPersonBP/Blueprints/FirstPersonProjectile.FirstPersonProjectile_C" (Transformation|GetWorldTransform (Variables|Default|GetProyectileSpawnLocation)) "Undefined" 0 0))
        (Physics|AddImpulse (Variables|/Game/FirstPersonBP/Blueprints/FirstPersonProjectile.FirstPersonProjectile_C|GetSphere _returnvalue) (* (Math|Vector|GetForwardVector (Variables|Default|GetCube)) (Variables|Default|GetShootAmount)) "None" true)
        (Variables|Default|SetProyectilSpawn false)
        (Utilities|FlowControl|Delay 1.5)
        (Variables|Default|SetProyectilSpawn true)))))

(event EventBeginPlay
  ;[1 1 1] PatrolPoint
  (Variables|Default|SetPatrolPoint (Utilities|Array|MakeArray (Transformation|GetWorldLocation (Variables|Default|GetMovePosition1)) (Transformation|GetWorldLocation (Variables|Default|GetMovePosition2)) (Transformation|GetWorldLocation (Variables|Default|GetMovePosition3))))
  (CallFunction|GetRandomLocation))

(event EventTakeDamage
  (params (Damage :type Float%20%28single-precision%29))
  (bind _output_get (Variables|Default|SetHealth (- (Variables|Default|GetHealth) Damage)))
  (if (<= _output_get 0.0)
    (Actor|DestroyActor)))

(fn ConstructionScript)

(fn GetRandomLocation
  (Variables|Default|SetCurrentPatrollPoint (Math|Random|RandomInteger (Utilities|Array|Length (Variables|Default|GetPatrolPoint)))))