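; BP_PlayerController is a player controller Blueprint that handles the player's death and restarts the game.
; On OnDeath it unpossesses the pawn, fades the camera out and holds it, and shows a BP_YouDied widget.
; After a short delay it removes the widget and calls RestartGame on the FirstPersonGameMode, provided the cast succeeds.
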(event Custom|OnDeath
  (Pawn|UnPossess)
  (CameraFades|StartCameraFade :self (Variables|Default|GetPlayerCameraManager) :ToAlpha 1.0 :Duration 1.0 :bHoldWhenFinished true)
  (bind _returnvalue (UserInterface|CreateWidget "/Game/Blueprints/BP_YouDied.BP_YouDied_C" self))
  (UserInterface|Viewport|AddtoViewport _returnvalue 0)
  (Utilities|FlowControl|Delay 2.0)
  (Widget|RemovefromParent _returnvalue)
  (bind _asfirst_person_game_mode (Utilities|Casting|CastToFirstPersonGameMode (Game|GetGameMode)))
  (Class|GameMode|RestartGame _asfirst_person_game_mode))

(event EventBeginPlay)

(event EventTick
  (params (DeltaSeconds :type Float%20%28single-precision%29)))

(fn ConstructionScript)