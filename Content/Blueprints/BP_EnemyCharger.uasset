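; BP_EnemyCharger is an enemy pawn that charges at the player and deals damage on contact.
; When PawnSensing sees a FirstPersonCharacter, AI MoveTo sends the pawn toward it.
; Any actor overlap sends a fixed TakeDamage message to that actor, with no filtering.
; Incoming damage lowers Health, but the zero-health branch is empty, so death is not handled.
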(event OnSeePawn(PawnSensing)
  (params (Pawn :type Pawn%20Object%20Reference))
  (bind _asfirst_person_character (Utilities|Casting|CastToFirstPersonCharacter Pawn))
  (AI|AIMoveTo self "0, 0, 0" _asfirst_person_character 5.0 false))

(event Collision|EventActorBeginOverlap
  (params (OtherActor :type Actor%20Object%20Reference))
  (Class|BPDamage|TakeDamage(Message) OtherActor 1e+01))

(event EventTakeDamage
  (params (Damage :type Float%20%28single-precision%29))
  (bind _output_get (Variables|Default|SetHealth (- (Variables|Default|GetHealth) Damage)))
  (if (<= _output_get 0.0)
    _))

(fn ConstructionScript)